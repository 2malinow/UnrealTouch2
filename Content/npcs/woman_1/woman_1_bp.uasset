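; Woman NPC Blueprint that moves its actor along the Weg spline of a referenced Track.
; On BeginPlay it sets Timeline0's play rate from the inverse of Duration, then plays Timeline_0 from the start.
; Each update maps the timeline's Alpha to a distance along the spline, applies that world location and rotation, then adds a fixed 90-degree local rotation offset.
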(event `self.ReceiveBeginPlay`
  (bind _weg (`/Game/Routen/Rundgang_dorf_5.Weg` (`self.track`)))
  (bind _returnvalue (`KismetMathLibrary.Lerp` 0.0 (`SplineComponent.GetSplineLength` _weg) (`self.Alpha`)))
  (`TimelineComponent.SetPlayRate` (`self.Timeline_0`) (/ 1.0 (`self.Duration`)))
  (bind (_direction _alpha) (`Timeline|Timeline_0` :!via `PlayFromStart`)
    (:`Update`
      (set `self.Alpha` _alpha)
      (`self.K2_SetActorLocationAndRotation` (`SplineComponent.GetLocationAtDistanceAlongSpline` _weg _returnvalue "World") (`SplineComponent.GetRotationAtDistanceAlongSpline` _weg _returnvalue "World"))
      (`self.K2_AddActorLocalRotation` (struct :`Yaw` -90.0)))))

(fn `UserConstructionScript`)