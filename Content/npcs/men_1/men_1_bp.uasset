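; Blueprint for the men_1 NPC that moves it along the Weg spline of a referenced Track actor.
; On BeginPlay it sets the timeline play rate from Duration and starts playback time at a fixed offset.
; Each timeline update maps Alpha to spline distance, applies that world location and rotation, then adds a fixed yaw correction to orient the character.
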(event `self.ReceiveBeginPlay`
  (bind _weg (`/Game/Routen/Rundgang_dorf.Weg` (`self.track`)))
  (bind _returnvalue (`KismetMathLibrary.Lerp` 0.0 (`SplineComponent.GetSplineLength` _weg) (`self.Alpha`)))
  (`TimelineComponent.SetPlayRate` (`self.Timeline_0`) (/ 1.0 (`self.Duration`)))
  (`TimelineComponent.SetNewTime` (`self.Timeline_0`) 0.7)
  (bind (_direction _alpha) (`Timeline|Timeline_0`)
    (:`Update`
      (set `self.Alpha` _alpha)
      (`self.K2_SetActorLocationAndRotation` (`SplineComponent.GetLocationAtDistanceAlongSpline` _weg _returnvalue "World") (`SplineComponent.GetRotationAtDistanceAlongSpline` _weg _returnvalue "World"))
      (`self.K2_AddActorLocalRotation` (struct :`Yaw` -90.0)))))

(fn `UserConstructionScript`)