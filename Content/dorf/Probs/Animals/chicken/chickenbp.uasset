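; Chicken animal actor that wanders between TargetPoints placed in the level.
; BeginPlay caches the TargetPoints and its start location, and Tick re-enters the same proximity check every frame.
; When near its stored location, it pauses randomly, picks one of the first ten points and glides there with an eased MoveComponentTo of random duration.
; No navigation or AI movement is used.
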(event `self.ReceiveBeginPlay`
  (bind _outactors (`GameplayStatics.GetAllActorsOfClass` "/Game/dorf/Probs/Animals/chicken/TargetPoint.TargetPoint_C"))
  (set `self.location` (`self.K2_GetActorLocation`))
  (if (== (`self.K2_GetActorLocation`) (`self.location`) :`ErrorTolerance` 50.0) :!label _label
    (`KismetSystemLibrary.Delay` (`KismetMathLibrary.RandomFloatInRange` 5.0 10.0))
    (bind _output_get (set `self.location` (`self.K2_GetActorLocation` (`|GetArrayItem` _outactors (`KismetMathLibrary.RandomIntegerInRange` 0 9)))))
    (`KismetSystemLibrary.MoveComponentTo` (`self.RootComponent`) _output_get (struct) true true (`KismetMathLibrary.RandomFloatInRange` 4.0 10.0))
    (set `self.location` (`self.K2_GetActorLocation`))))

(event `self.ReceiveTick`
  (params (DeltaSeconds :type "Float (single-precision)"))
  (goto _label))

(fn `UserConstructionScript`)